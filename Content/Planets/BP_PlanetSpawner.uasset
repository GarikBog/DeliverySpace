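; Planet spawner that periodically creates fish-wanting planets inside a box, each with a random order from the unlocked items.
; A looping timer spawns while the box's overlap count is under the cap, teleporting a probe sphere randomly until it finds a clear spot.
; Each planet receives a spawner reference.
; Repeated completed orders of the current item advance the unlock progression, which opens the "Developers" level once the item list runs out.
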(event Custom|StartSpawn
  (Utilities|Time|SetTimerbyEvent (delegate Custom|SpawnPlanet) (Variables|Default|GetSpawnDelay) true)
  (Utilities|FlowControl|Delay 1.0)
  (CallFunction|SpawnPlanet))

(event Custom|SpawnPlanet
  (bind _box (Variables|Default|GetBox))
  (bind _sphere (Variables|Default|GetSphere))
  (bind _returnvalue (Transformation|GetWorldLocation _box))
  (bind _returnvalue_2 (Components|Box|GetScaledBoxExtent _box))
  (bind _returnvalue_3 (Math|Random|RandomPointinBoundingBox _returnvalue _returnvalue_2))
  (if (< (CallFunction|GetPlanetsIs) 9)
    (while (!= (Utilities|Array|Length (Collision|GetOverlappingActors _sphere 0 :!class /Script/Engine.PrimitiveComponent)) 1)
      (Transformation|SetWorldLocation _sphere (Math|Vector|MakeVector (.x _returnvalue_3) (.y _returnvalue_3) 0.0) false true))
    (bind _returnvalue_4 (Game|SpawnActorfromClass "/Game/Planets/Planets/BP_PlanetWhoWantsFish.BP_PlanetWhoWantsFish_C" (Math|Transform|MakeTransform (Transformation|GetWorldLocation _sphere) "0, 0, 0" "1.000000,1.000000,1.000000") "Undefined" "MultiplyWithRoot" 0 0))
    (Default|SetOrder _returnvalue_4 (CallFunction|GetRandomItem))
    (Class|BPIPlanetsandSpawner|YouAreNew(Message) _returnvalue_4 self)))

(event EventBeginPlay
  (bind _allitems (Variables|Default|GetAllItems))
  (bind _output (Utilities|Array|Get(acopy) _allitems))
  (CallFunction|StartSpawn)
  (Utilities|Array|Add (Variables|Default|GetAvailableItems) _output)
  (Variables|Default|SetCurrentItem _output))

(event EventNewOrderComplited
  (params (PlanetOrder :type BP%20Item%20Base%20Class%20Reference))
  (bind _next (Variables|Default|GetNext))
  (bind _allitems (Variables|Default|GetAllItems))
  (bind _output (Utilities|Array|Get(acopy) _allitems _next))
  (if (== PlanetOrder (Variables|Default|GetCurrentItem))
    (bind _result (Math|Integer|IncrementInt (Variables|Default|GetNewOrdersComplite))
      (:%20%20
        (if (== _result 5)
          (Utilities|Array|Add (Variables|Default|GetAvailableItems) _output)
          (bind _result_2 (Math|Integer|IncrementInt _next)
            (:%20%20
              (if (> _result_2 (Utilities|Array|Length _allitems))
                (Game|OpenLevel(byName) "Developers")
                (else
                  (Variables|Default|SetCurrentItem _output)
                  (Variables|Default|SetNewOrdersComplite 0))))))))))

(event EventTick
  (params (DeltaSeconds :type Float%20%28single-precision%29)))

(fn ConstructionScript)

(fn GetRandomItem
  (bind _availableitems (Variables|Default|GetAvailableItems))
  (return (Utilities|Array|Get(acopy) _availableitems (Math|Random|RandomInteger (Utilities|Array|Length _availableitems)))))

(fn GetPlanetsIs
  (return (- (Utilities|Array|Length (Collision|GetOverlappingActors (Variables|Default|GetBox) 0 :!class /Script/Engine.PrimitiveComponent)) 2)))