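; Base planet actor that shows an order widget and trades the player ship's requested item for award items and gold.
; Clicking the widget sends the ship here, or completes the order if already in orbit and notifies the Spawner.
; Cross-resetting DoOnce nodes gate overlap-driven arrival and departure; completed planets self-destroy after departure and a delay unless targeted.
; Helpers configure the order, award and pirate mesh, and compute four orbit points.
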(event OnComponentBeginOverlap(CollisionForIntefraceInteract)
  (params (OverlappedComponent :type Primitive%20Component%20Object%20Reference) (OtherActor :type Actor%20Object%20Reference) (OtherComp :type Primitive%20Component%20Object%20Reference) (OtherBodyIndex :type Integer) (bFromSweep :type Boolean) (SweepResult :type Hit%20Result%20Structure%20%28by%20ref%29))
  (if (Actor|ActorHasTag OtherActor "Ship")
    (Utilities|FlowControl|DoOnce false
      (:Completed
        (CallFunction|ShipArrivesPlanet)
        (Utilities|FlowControl|DoOnce false) ; enters at Reset
      ))))

(event OnComponentEndOverlap(CollisionForIntefraceInteract)
  (params (OverlappedComponent :type Primitive%20Component%20Object%20Reference) (OtherActor :type Actor%20Object%20Reference) (OtherComp :type Primitive%20Component%20Object%20Reference) (OtherBodyIndex :type Integer))
  (if (Actor|ActorHasTag OtherActor "Ship")
    (Utilities|FlowControl|DoOnce false
      (:Completed
        (CallFunction|ShipLeavingPlanet)
        (Utilities|FlowControl|DoOnce false) ; enters at Reset
      ))))

(event Custom|OrderComplete
  (bind _returnvalue (Game|Player|GetPlayerPawn 0))
  ;[0.15 0.15 0.15 0.5] OrderComplete
  (if (Variables|Default|GetbShipOnOrbite)
    (bind _bisgive (Class|BPIShipandPlanetInteract|RequestFood(Message) _returnvalue (Variables|Default|GetOrder)))
    (if _bisgive
      (Class|BPIShipandPlanetInteract|GiveAward(Message) _returnvalue (Variables|Default|GetCompleteAward) (Variables|Default|GetGoldAward))
      (Variables|Default|SetbIsOrderComplited true)
      (Widget|SetVisibility (Variables|Default|GetPlanetOrderWidget) "Hidden")
      (Class|BPIPlanetsandSpawner|NewOrderComplited(Message) (Variables|Default|GetSpawner) (Variables|Default|GetOrder))
      (else
        (Audio|PlaySound2D "/Game/Sounds/Cutted/noNeededItem_cut_.noNeededItem_cut_" 1.0 1.0 0.0 0 0)))
    (else
      (bind _asbp_ship (Utilities|Casting|CastToBP_Ship (Game|Player|GetPlayerPawn 0)))
      (Default|MovetoPlanet _asbp_ship self))))

(event EventBeginPlay
  ;[0.15 0.15 0.15 0.5] Begin Play
  (Audio|PlaySound2D "/Game/Sounds/pelemeni_warp_1.pelemeni_warp_1" 1.0 1.0 0.0 0 0)
  (bind _returnvalue (UserInterface|CreateWidget "/Game/UI_UX/Widgets/WBP_PlanetOrder.WBP_PlanetOrder_C"))
  (Variables|Default|SetPlanetOrderWidget _returnvalue)
  (EventDispatchers|BindEventtoButtonWasClicked _returnvalue (delegate Custom|OrderComplete)))

(event EventYouAreNew
  (params (Spawner :type BP%20Planet%20Spawner%20Object%20Reference))
  (Variables|Default|SetbIsNew true)
  (Variables|Default|SetSpawner Spawner))

(event EventShowOrder
  ;[0.15 0.15 0.15 0.5] Events ShowOrder And GideOrder
  (if (not (Variables|Default|GetbIsOrderComplited))
    (Widget|SetVisibility (Variables|Default|GetPlanetOrderWidget) "Visible")
    (Utilities|FlowControl|Delay 2.0)
    (CallFunction|HideOrder)))

(event EventHideOrder
  ;[0.15 0.15 0.15 0.5] Events ShowOrder And GideOrder
  (if (not (Variables|Default|GetbShipOnOrbite))
    (Widget|SetVisibility (Variables|Default|GetPlanetOrderWidget) "Hidden")))

(event EventShipLeavingPlanet
  (Variables|Default|SetbShipOnOrbite false)
  (CallFunction|HideOrder)
  (if (Variables|Default|GetbIsOrderComplited)
    (Utilities|FlowControl|Delay (Variables|Default|GetDelayToHidePlanet))
    (if (not (Variables|Default|GetbIsTarget))
      (Audio|PlaySound2D "/Game/Sounds/pelemeni_warp_2.pelemeni_warp_2" 1.0 1.0 0.0 0 0)
      (Actor|DestroyActor))))

(event EventShipArrivesPlanet
  (Variables|Default|SetbShipOnOrbite true)
  (CallFunction|ShowOrder))

(fn ConstructionScript)

(fn GetOrbitPoses
  (bind _planetcollision (Variables|Default|GetPlanetCollision))
  (bind _newlocalvar (LocalVariables|GetNewLocalVar))
  (bind _returnvalue (Transformation|GetWorldLocation _planetcollision))
  (bind _sphereradius (Variables|/Script/Engine.SphereComponent|GetSphereRadius _planetcollision))
  (bind _returnvalue_2 (+ _sphereradius 15.0))
  (Utilities|Array|Add _newlocalvar (Math|Vector|MakeVector (+ (.x _returnvalue) _returnvalue_2) (.y _returnvalue) (.z _returnvalue)))
  (Utilities|Array|Add _newlocalvar (Math|Vector|MakeVector (- (.x _returnvalue) _returnvalue_2) (.y _returnvalue) (.z _returnvalue)))
  (Utilities|Array|Add _newlocalvar (Math|Vector|MakeVector (.x _returnvalue) (+ (.y _returnvalue) _returnvalue_2) (.z _returnvalue)))
  (Utilities|Array|Add _newlocalvar (Math|Vector|MakeVector (.x _returnvalue) (- (.y _returnvalue) _returnvalue_2) (.z _returnvalue)))
  (return (LocalVariables|GetNewLocalVar)))

(fn CreateOrderWidget
  (params (Order :type BP%20Item%20Base%20Class%20Reference))
  (bind _planetorderwidget (Variables|Default|GetPlanetOrderWidget))
  (bind _returnvalue (Game|SpawnActorfromClass Order (Math|Transform|MakeTransform "0, 0, 0" "0, 0, 0" "1.000000,1.000000,1.000000") "Undefined" "MultiplyWithRoot" 0 0))
  (Variables|Default|SetCompleteAward (Variables|/Game/Items/BP_ItemBase.BP_ItemBase_C|GetItemsInAward _returnvalue))
  (Variables|/Game/UI_UX/Widgets/WBP_PlanetOrder.WBP_PlanetOrder_C|SetImage _planetorderwidget (Variables|/Game/Items/BP_ItemBase.BP_ItemBase_C|GetItemImage _returnvalue))
  (Variables|Default|SetGoldAward (Variables|/Game/Items/BP_ItemBase.BP_ItemBase_C|GetCostAsAward _returnvalue))
  (Variables|/Game/UI_UX/Widgets/WBP_PlanetOrder.WBP_PlanetOrder_C|SetPlayerActor _planetorderwidget self)
  (UserInterface|Viewport|AddtoViewport _planetorderwidget 0)
  (Widget|SetVisibility _planetorderwidget "Hidden"))

(fn SetPirate
  (params (bIsPirate :type Boolean))
  (Variables|Default|SetbIsPirate bIsPirate)
  (Development|SetHiddeninGame (Variables|Default|GetPirateShipMesh) (not bIsPirate) false))

(fn SetAward
  (params (Items :type Array%20of%20BP%20Item%20Base%20Class%20References))
  (Variables|Default|SetCompleteAward Items))

(fn SetOrder
  (params (Item :type BP%20Item%20Base%20Class%20Reference))
  (bind _output_get (Variables|Default|SetOrder Item))
  (CallFunction|CreateOrderWidget _output_get))

(fn RequestFood
  (params (Item :type BP%20Item%20Base%20Class%20Reference))
  (return false))