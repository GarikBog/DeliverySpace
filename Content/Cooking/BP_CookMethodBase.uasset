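; BP_CookMethodBase is a cooking method base that runs an arrow-key sequence minigame.
; StartCook takes the cooking display from the main HUD and starts a looping timer, whose tick is gated by a DoOnce that each ButtonPressed resets.
; CheckArrow compares the press with the Keys entry at CurrentIndex, driving right or wrong messages.
; The last correct key shows success, stops the timer and resets the index to 1.
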(event Custom|CookTick
  (bind _cookdisplay (Variables|Default|GetCookDisplay))
  ;[0.15 0.15 0.15 0.5] Cook
  (Utilities|FlowControl|DoOnce true
    (:Completed
      (bind (_bisright _bislast) (CallFunction|CheckArrow))
      (if _bisright
        (Class|BPICookInteractwithCookMethod|RightButton(Message) _cookdisplay)
        (if _bislast
          (Variables|Default|SetbIsActive false)
          (Class|BPICook|CookSuccess(Message) (stale EventStartCook _aswbp_main_hud))
          (Utilities|Time|ClearandInvalidateTimerbyHandle (stale EventStartCook _returnvalue))
          (Variables|Default|SetCurrentIndex 1)
          (else
            (Math|Integer|IncrementInt (Variables|Default|GetCurrentIndex)
              (:%20%20
                (Variables|Default|SetLastPressedArrow "None")))))
        (else
          (Class|BPICookInteractwithCookMethod|WrongButton(Message) _cookdisplay))))))

(event EventBeginPlay
  (Input|AddMappingContext (PlayerController|LocalPlayerSubsystems|GetEnhancedInputLocalPlayerSubsystem (Game|GetPlayerController 0)) "/Game/Inputs/IMC_Standart.IMC_Standart" 0 "(bIgnoreAllPressedKeysUntilRelease=True,bForceImmediately=False,bNotifyUserSettings=False)"))

(event EventStartCook
  (params (FromClass :type Object%20Object%20Reference))
  ;[0.15 0.15 0.15 0.5] Cook
  (bind _aswbp_main_hud (Utilities|Casting|CastToWBP_MainHUD FromClass))
  (Variables|Default|SetbIsActive true)
  (Variables|Default|SetCookDisplay (Variables|/Game/UI_UX/WBP_MainHUD.WBP_MainHUD_C|GetWBP_Cooking _aswbp_main_hud))
  (bind _returnvalue (Utilities|Time|SetTimerbyEvent (delegate Custom|CookTick) 0.1 true)))

(event EventButtonPressed
  (params (Key :type Key%20Structure :default "None"))
  (bind _cookdisplay (Variables|Default|GetCookDisplay))
  ;[0.15 0.15 0.15 0.5] Last Pressed Arrow
  (if (Variables|Default|GetbIsActive)
    (Variables|Default|SetLastPressedArrow Key)
    ;[0.15 0.15 0.15 0.5] Cook
    (Utilities|FlowControl|DoOnce true) ; enters at Reset
  ))

(fn ConstructionScript)

(fn CheckArrow
  (bind _keys (Variables|Default|GetKeys))
  (bind _currentindex (Variables|Default|GetCurrentIndex))
  (return (== (Utilities|Array|Get(acopy) _keys _currentindex) (Variables|Default|GetLastPressedArrow)) (>= _currentindex (- (Utilities|Array|Length _keys) 1))))

(fn FirstArrow
  (return (Utilities|Array|Get(acopy) (Variables|Default|GetKeys))))