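; BP_RecipeBook is the cooking recipe book that stores recipes and finds the one matching a set of items.
; AddRecipe spawns a recipe actor from a class and files it into the Up, Down, Left or Right array by its first arrow.
; Each direction has a Find function that returns the first recipe whose CompareItems accepts the items.
; BeginPlay calls AddBaseRecipes, which is empty here.
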(event EventBeginPlay
  (CallFunction|AddBaseRecipes))

(fn ConstructionScript)

(fn FindRecipeUp
  (params (Items :type Array%20of%20BP%20Item%20Base%20Object%20References))
  (for _array_element (Variables|Default|GetRecipes_Up)
    (bind _bissuitable_ (Default|CompareItems _array_element Items))
    (if _bissuitable_
      (return _array_element)))
  (return 0))

(fn FindRecipeDown
  (params (Items :type Array%20of%20BP%20Item%20Base%20Object%20References))
  (for _array_element (Variables|Default|GetRecipes_Down)
    (bind _bissuitable_ (Default|CompareItems _array_element Items))
    (if _bissuitable_
      (return _array_element)))
  (return 0))

(fn FindRecipeLeft
  (params (Items :type Array%20of%20BP%20Item%20Base%20Object%20References))
  (for _array_element (Variables|Default|GetRecipes_Left)
    (bind _bissuitable_ (Default|CompareItems _array_element Items))
    (if _bissuitable_
      (return _array_element)))
  (return 0))

(fn FindRecipeRight
  (params (Items :type Array%20of%20BP%20Item%20Base%20Object%20References))
  (for _array_element (Variables|Default|GetRecipes_Right)
    (bind _bissuitable_ (Default|CompareItems _array_element Items))
    (if _bissuitable_
      (return _array_element)))
  (return 0))

(fn AddBaseRecipes)

(fn AddRecipe
  (params (Recipe :type BP%20Recipe%20Base%20Class%20Reference))
  (bind _returnvalue (Game|SpawnActorfromClass Recipe (Math|Transform|MakeTransform "0, 0, 0" "0, 0, 0" "1.000000,1.000000,1.000000") "Undefined" "MultiplyWithRoot" 0 0))
  (if (== (Default|GetFirstArrow _returnvalue) "Up")
    (Utilities|Array|Add (Variables|Default|GetRecipes_Up) _returnvalue)
    (elif (== (Default|GetFirstArrow _returnvalue) "Down")
      (Utilities|Array|Add (Variables|Default|GetRecipes_Down) _returnvalue)
      (elif (== (Default|GetFirstArrow _returnvalue) "Left")
        (Utilities|Array|Add (Variables|Default|GetRecipes_Left) _returnvalue)
        (else
          (Utilities|Array|Add (Variables|Default|GetRecipes_Right) _returnvalue))))))