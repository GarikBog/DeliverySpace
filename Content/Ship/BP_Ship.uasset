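; BP_Ship is the player's click-to-move ship, which travels between planets and links their food orders and rewards to the main HUD.
; BeginPlay sets the view to a level CameraActor, adds input mapping, shows the cursor and creates the HUD.
; Cursor traces find tagged interface planets: a looping timer shows the hovered planet's order, and clicking targets one, using SimpleMoveToLocation toward its last orbit position.
; GiveAward and RequestFood forward to the HUD.
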(event Custom|CheckPlanet
  (bind _planet (CallFunction|GetPlanetUnderMouse))
  (if (not (Variables|/Game/UI_UX/WBP_MainHUD.WBP_MainHUD_C|GetbAwardIsOpen (Variables|Default|GetHUD)))
    (Utilities|IsValid _planet
      (:Is%20Valid
        (Class|BPIShipandPlanetInteract|ShowOrder(Message) _planet)))))

(event EventBeginPlay
  (bind _returnvalue (Game|GetPlayerController 0))
  (bind _outactors (Actor|GetAllActorsOfClass "/Script/Engine.CameraActor"))
  (for _array_element _outactors
    (bind _output_get (Variables|Default|SetCamera _array_element))
    (Game|Player|SetViewTargetwithBlend (Game|GetPlayerController 0) _output_get 0.0 "VTBlend_Linear" 0.0 false)
    (Input|AddMappingContext (PlayerController|LocalPlayerSubsystems|GetEnhancedInputLocalPlayerSubsystem _returnvalue) "/Game/Inputs/IMC_Standart.IMC_Standart" 0 "(bIgnoreAllPressedKeysUntilRelease=True,bForceImmediately=False,bNotifyUserSettings=False)")
    (Variables|/Script/Engine.PlayerController|SetbShowMouseCursor _returnvalue true)
    (bind _returnvalue_2 (UserInterface|CreateWidget "/Game/UI_UX/WBP_MainHUD.WBP_MainHUD_C"))
    (bind _output_get_2 (Variables|Default|SetHUD _returnvalue_2))
    (UserInterface|Viewport|AddtoViewport _output_get_2 0)
    (Utilities|Time|SetTimerbyEvent (delegate Custom|CheckPlanet) 0.1 true)))

(event EventGiveAward
  (params (Items :type Array%20of%20BP%20Item%20Base%20Class%20References) (Gold :type Integer))
  (bind _hud (Variables|Default|GetHUD))
  (Variables|/Game/UI_UX/WBP_MainHUD.WBP_MainHUD_C|SetGoldAward _hud Gold)
  (Default|RefreshChoise _hud Items))

(event Input|MouseEvents|LeftMouseButton
  (params (Key :type Key%20Structure :default "None"))
  (:Released
    (if (Variables|Default|GetbIsCanMoving)
      (CallFunction|MovetoPlanet (CallFunction|GetPlanetUnderMouse)))))

(fn ConstructionScript)

(fn MovetoPlanet
  (params (Planet :type Actor%20Object%20Reference))
  (if (Variables|Default|GetbIsCanMoving)
    (Utilities|IsValid (Variables|Default|GetPlanetBased)
      (:Is%20Valid
        (Variables|/Game/Planets/BP_PlanetBase.BP_PlanetBase_C|SetbIsTarget (Variables|Default|GetPlanetBased) false))
      (:Is%20Not%20Valid
        _))
    (bind _asbp_planet_base (Utilities|Casting|CastToBP_PlanetBase Planet))
    (bind _output_get (Variables|Default|SetPlanetBased _asbp_planet_base))
    (Variables|/Game/Planets/BP_PlanetBase.BP_PlanetBase_C|SetbIsTarget _output_get true)
    (bind _newparam (Default|GetOrbitPoses _output_get))
    (for _array_element _newparam
      _)
    (AI|Navigation|SimpleMovetoLocation (Game|GetPlayerController 0) _array_element)))

(fn GetPlanetUnderMouse
  (bind _returnvalue (Game|GetPlayerController 0))
  (bind _hitresult (Game|Player|GetHitResultUnderCursorbyChannel _returnvalue "TraceTypeQuery1" true))
  (bind (_bblockinghit _binitialoverlap _time _distance _location _impactpoint _normal _impactnormal _physmat _hitactor) (Collision|BreakHitResult _hitresult))
  (Utilities|IsValid _hitactor
    (:Is%20Valid
      (if (Math|Boolean|ANDBoolean _bblockinghit (Actor|ActorHasTag _hitactor "Planet") (Utilities|DoesObjectImplementInterface _hitactor "/Game/Interfaces/Inventory/BPI_ShipAndPlanetInteract.BPI_ShipAndPlanetInteract_C"))
        (return _hitactor)
        (else
          (return 0))))))

(fn RequestFood
  (params (Item :type BP%20Item%20Base%20Class%20Reference))
  (bind _bisgive (Default|GiveOrder (Variables|Default|GetHUD) Item))
  (return _bisgive))